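; Game mode for Bumper Brawl, a local multiplayer car game that spawns and possesses a SportsCar pawn at each PlayerStart, creating extra players from numeric tags.
; Tick derives one-frame pause/resume flags and compares input device count to local players, with inverted EnoughLocalControllers naming.
; The ControllerDisconnected widget is removed when devices suffice, but its show logic is unwired.
; Eliminations are recorded, but winner and round-win logic are stubs.
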(event `self.ReceiveBeginPlay`
  (bind _returnvalue (`GameplayStatics.GetPlayerController` 0))
  (set `self.FirstFrame` true)
  (bind _output_get (set `self.EnoughLocalControllers` true))
  (set `self.LastControllerState` _output_get)
  (bind _output_get_2 (set `self.Paused` false))
  (set `self.lastPauseState` _output_get_2)
  (set `self.OnPauseFrame` false)
  (set `self.OnResumeFrame` false)
  (bind _outactors (`GameplayStatics.GetAllActorsOfClass` "/Script/Engine.PlayerStart"))
  (for _array_element _outactors
    (bind _returnvalue_2 (`KismetStringLibrary.Conv_StringToInt` (`KismetStringLibrary.Conv_NameToString` (`PlayerStart.PlayerStartTag` _array_element))))
    (if (> _returnvalue_2 0)
      (bind _returnvalue_3 (`GameplayStatics.CreatePlayer` _returnvalue_2))
      (bind _returnvalue_4 (`self.GetTransform` _array_element))
      (bind _returnvalue_5 (`|SpawnActorFromClass` "/Game/Blueprints/PlayerBlueprints/SportsCar_Pawn.SportsCar_Pawn_C" _returnvalue_4 "Undefined" "MultiplyWithRoot" null null))
      (`Controller.Possess` _returnvalue_3 _returnvalue_5)
      (else
        (bind _returnvalue_6 (`|SpawnActorFromClass` "/Game/Blueprints/PlayerBlueprints/SportsCar_Pawn.SportsCar_Pawn_C" _returnvalue_4 "Undefined" "MultiplyWithRoot" _returnvalue null))
        (`Controller.Possess` _returnvalue _returnvalue_6)
        (bind _returnvalue_7 (`|CreateWidget` "/Game/Blueprints/UI/ControllerDisconnected.ControllerDisconnected_C" _returnvalue))
        (set `self.UI Reference` _returnvalue_7)))))

(event `PlayerEliminated`
  (params (ElliminatedPlayer :type "Pawn Object Reference"))
  (`KismetArrayLibrary.Array_Add` (`self.EliminatedPlayers`) ElliminatedPlayer)
  (`self.CheckWinner`))

(event `CheckWinner`
  (`GameplayStatics.GetActorOfClass` "/Game/Blueprints/PlayerBlueprints/VehicleAdvPawn.VehicleAdvPawn_C")
  (for _ (`self.EliminatedPlayers`)
    _))

(event `WinRound`
  (params (NewParam :type "Array of Pawn Object Reference")))

(event `self.ReceiveTick`
  (params (DeltaSeconds :type "Float (single-precision)"))
  (`self.HandlePauseState`)
  (`self.checkNumControllers`)
  (set `self.LastControllerState` (`self.EnoughLocalControllers`)))

(fn `checkNumControllers`
  (bind _outinputdevices (`InputDeviceLibrary.GetAllConnectedInputDevices`))
  (if (< (`KismetArrayLibrary.Array_Length` _outinputdevices) (`GameplayStatics.GetNumLocalPlayerControllers`))
    (set `self.EnoughLocalControllers` true)
    (else
      (set `self.EnoughLocalControllers` false)
      (if (!= (`self.EnoughLocalControllers`) (`self.LastControllerState`))
        (`Widget.RemoveFromParent` (`self.UI Reference`))))))

(fn `HandlePauseState`
  (if (!= (`self.Paused`) (`self.lastPauseState`))
    (if (`self.Paused`)
      (set `self.OnPauseFrame` true)
      (set `self.OnResumeFrame` false)
      (else
        (set `self.OnPauseFrame` false)
        (set `self.OnResumeFrame` true)))
    (else
      (set `self.OnPauseFrame` false)
      (set `self.OnResumeFrame` false)))
  (set `self.lastPauseState` (`self.Paused`)))

(fn `UserConstructionScript`)