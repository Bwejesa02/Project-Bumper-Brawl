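; Bumper Brawl safezone that blows up vehicles caught outside it when each stage timer expires.
; Sphere overlaps, with a center-distance check on entry, maintain the array of vehicles inside.
; Tick counts down unless the gamemode is paused, playing an audio clock tick each second.
; At stage end it explodes and destroys outsiders; if anyone is inside, the timer resets and the zone jumps to a random marker after a delay.
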(event `self.ReceiveBeginPlay`
  (bind _returnvalue (`GameplayStatics.GetActorOfClass` "/Game/Blueprints/BP_GamemodeBumperBrawl.BP_GamemodeBumperBrawl_C"))
  (set `self.gamemode` _returnvalue)
  (bind _returnvalue_2 (`FMODBlueprintStatics.PlayEvent2D` "/Game/FMOD/Events/ClockTick.ClockTick"))
  (set `self.ClockTick` _returnvalue_2)
  (set `self.LastStageTimerSeconds` 30))

(event `ResetSafeZone`
  (bind _safezonemarkers (`self.SafezoneMarkers`))
  ;[0 0 0] Position Reset
  (set `self.StageTimer` 30.0)
  (`KismetSystemLibrary.Delay` 3.0)
  (`SceneComponent.K2_SetWorldLocation` (`self.DefaultSceneRoot`) (`self.K2_GetActorLocation` (`|GetArrayItem` _safezonemarkers (`KismetMathLibrary.RandomIntegerInRange` 0 (- (`KismetArrayLibrary.Array_Length` _safezonemarkers) 1)))) false false)
  (bind _output_get (set `self.ExplodeInstance` (struct)))
  (`FMODBlueprintStatics.EventInstanceRelease` _output_get))

(event `self.ReceiveTick`
  (params (DeltaSeconds :type "Float (single-precision)"))
  ;[0 0 0] Timer for Safezone stages
  (if (not (`/Game/Blueprints/BP_GamemodeBumperBrawl.paused` (`self.gamemode`)))
    (bind _output_get (set `self.StageTimer` (- (`self.StageTimer`) DeltaSeconds)))
    (`self.PlayClockTick` _output_get)
    (if (<= (`self.StageTimer`) 0.0)
      (`self.OnStageEnd`))))

(event `OnStageEnd`
  ;[0 0 0] Stage End - Destroys players out of safezone
  (if (not (`/Game/Blueprints/BP_GamemodeBumperBrawl.paused` (`self.gamemode`)))
    (bind _outactors (`GameplayStatics.GetAllActorsOfClass` "/Game/Blueprints/PlayerBlueprints/VehicleAdvPawn.VehicleAdvPawn_C"))
    (for _array_element _outactors
      (bind _asvehicle_adv_pawn (cast `/Game/Blueprints/PlayerBlueprints/VehicleAdvPawn` _array_element))
      (if (not (`KismetArrayLibrary.Array_Contains` (`self.PlayersInSafezone`) _asvehicle_adv_pawn))
        (`/Game/Blueprints/PlayerBlueprints/VehicleAdvPawn.releaseEngineSound` _asvehicle_adv_pawn)
        (bind (_returnvalue_location _returnvalue_rotation) (`KismetMathLibrary.BreakTransform` (`self.GetTransform` _asvehicle_adv_pawn)))
        (`GameplayStatics.SpawnEmitterAtLocation` "/Game/Assets/StarterContent/Particles/P_Explosion.P_Explosion" _returnvalue_location _returnvalue_rotation (2.0 2.0 1.0))
        (bind _returnvalue (`FMODBlueprintStatics.PlayEventAtLocation` "/Game/FMOD/Events/ExplodedDialogue.ExplodedDialogue" (`self.GetTransform` _asvehicle_adv_pawn)))
        (set `self.ExplodeInstance` _returnvalue)
        (`KismetSystemLibrary.Delay` 2.0)
        (`self.K2_DestroyActor` _asvehicle_adv_pawn)))
    (if (>= (`KismetArrayLibrary.Array_Length` (`self.PlayersInSafezone`)) 1)
      (`self.ResetSafeZone`))))

(event `self.SafezoneCollision.OnComponentBeginOverlap`
  (params (OverlappedComponent :type "PrimitiveComponent Object Reference") (OtherActor :type "Actor Object Reference") (OtherComp :type "PrimitiveComponent Object Reference") (OtherBodyIndex :type Integer) (bFromSweep :type Boolean) (SweepResult :type "HitResult Structure (by ref)"))
  ;[0 0 0] Checks if center of player is inside the Safezone - Adds to Array (PlayersInSafezone)
  (bind _asvehicle_adv_pawn (cast `/Game/Blueprints/PlayerBlueprints/VehicleAdvPawn` OtherActor))
  (if (>= (* (`SphereComponent.SphereRadius` (`self.SafezoneCollision`)) 1.1) (`KismetMathLibrary.VSize` (- (`self.K2_GetActorLocation` _asvehicle_adv_pawn) (`SceneComponent.K2_GetComponentLocation` (`self.SafezoneCollision`)))))
    (`KismetArrayLibrary.Array_AddUnique` (`self.PlayersInSafezone`) _asvehicle_adv_pawn)))

(event `self.SafezoneCollision.OnComponentEndOverlap`
  (params (OverlappedComponent :type "PrimitiveComponent Object Reference") (OtherActor :type "Actor Object Reference") (OtherComp :type "PrimitiveComponent Object Reference") (OtherBodyIndex :type Integer))
  ;[0 0 0] Checks if center of player has left the Safezone - Removes from array
  (bind _asvehicle_adv_pawn (cast `/Game/Blueprints/PlayerBlueprints/VehicleAdvPawn` OtherActor))
  (`KismetArrayLibrary.Array_RemoveItem` (`self.PlayersInSafezone`) _asvehicle_adv_pawn))

(event `self.ReceiveEndPlay`
  (params (EndPlayReason :type "EEndPlayReason Enum" :default "Destroyed"))
  (`FMODBlueprintStatics.EventInstanceRelease` (`self.ClockTick`)))

(fn `Get2DClockTick`
  (bind _returnvalue (`FMODBlueprintStatics.EventInstanceIsValid` (`self.ClockTick`)))
  (if (not _returnvalue)
    (`FMODBlueprintStatics.EventInstanceRelease` (`self.ClockTick`))
    (bind _returnvalue_2 (`FMODBlueprintStatics.PlayEvent2D` "/Game/FMOD/Events/ClockTick.ClockTick" false))
    (set `self.ClockTick` _returnvalue_2)))

(fn `PlayClockTick`
  (params (TimeSecond :type "Float (double-precision)"))
  (bind _returnvalue (`KismetMathLibrary.FFloor` TimeSecond))
  (if (!= _returnvalue (`self.LastStageTimerSeconds`))
    (`FMODBlueprintStatics.EventInstancePlay` (`self.ClockTick`)))
  (set `self.LastStageTimerSeconds` _returnvalue)
  (`self.Get2DClockTick`))

(fn `UserConstructionScript`)