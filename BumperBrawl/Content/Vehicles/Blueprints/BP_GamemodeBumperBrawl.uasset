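; BP_GamemodeBumperBrawl is the Bumper Brawl game mode that sets up local multiplayer sports car players at level start.
; On BeginPlay it loops over every PlayerStart and reads its PlayerStartTag as an integer controller index.
; Positive indices create a new local player, which possesses a SportsCar_Pawn spawned at that start.
; Any other tag spawns a car there and gives it to player controller 0.
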(event `self.ReceiveBeginPlay`
  (bind _returnvalue (`GameplayStatics.GetPlayerController` 0))
  (bind _outactors (`GameplayStatics.GetAllActorsOfClass` "/Script/Engine.PlayerStart"))
  (for _array_element _outactors
    (bind _returnvalue_2 (`KismetStringLibrary.Conv_StringToInt` (`KismetStringLibrary.Conv_NameToString` (`PlayerStart.PlayerStartTag` _array_element))))
    (if (> _returnvalue_2 0)
      (bind _returnvalue_3 (`GameplayStatics.CreatePlayer` _returnvalue_2))
      (bind _returnvalue_4 (`self.GetTransform` _array_element))
      (bind _returnvalue_5 (`|SpawnActorFromClass` "/Game/Vehicles/SportsCar/InstanceAssets/SportsCar_Pawn.SportsCar_Pawn_C" _returnvalue_4 "Undefined" "MultiplyWithRoot" null null))
      (`Controller.Possess` _returnvalue_3 _returnvalue_5)
      (else
        (bind _returnvalue_6 (`|SpawnActorFromClass` "/Game/Vehicles/SportsCar/InstanceAssets/SportsCar_Pawn.SportsCar_Pawn_C" _returnvalue_4 "Undefined" "MultiplyWithRoot" _returnvalue null))
        (`Controller.Possess` _returnvalue _returnvalue_6)))))

(fn `UserConstructionScript`)